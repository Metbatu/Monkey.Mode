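; BP_HumanSeen is a map actor whose Cube is shown or hidden according to its State enum, apparently as an object meant to be seen by humans.
; On BeginPlay it compares State to the first enum entry, making the Cube and its children visible on a match and hidden otherwise.
; Either way, Cube collision and component tick are disabled, and nothing re-evaluates the state afterward.
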(event `self.ReceiveBeginPlay`
  (bind _cube (`self.Cube`))
  (bind _cube_2 (`self.Cube`))
  (bind _returnvalue (`|EnumEquality` (`self.State`) "NewEnumerator0"))
  (for _ (`|MakeArray` _returnvalue)
    (if _returnvalue
      (`SceneComponent.SetVisibility` (`self.Cube`) true true)
      (`PrimitiveComponent.SetCollisionEnabled` _cube_2 "NoCollision")
      (`ActorComponent.SetComponentTickEnabled` _cube_2 false)
      (else
        (`SceneComponent.SetVisibility` (`self.Cube`) false true)
        (`PrimitiveComponent.SetCollisionEnabled` _cube "NoCollision")
        (`ActorComponent.SetComponentTickEnabled` _cube false)))))

(fn `UserConstructionScript`)