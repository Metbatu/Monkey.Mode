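; Lights actor that lets a player or other actor switch four spotlights off and on through interaction.
; Overlapping its Trigger component sends the other actor an interact-area enter message carrying a self reference, and leaving sends an exit message.
; The Interaction event drives a FlipFlop that alternates the spotlights' intensity between zero and full, starting with off.
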(event `self.Trigger.OnComponentBeginOverlap`
  (params (OverlappedComponent :type "PrimitiveComponent Object Reference") (OtherActor :type "Actor Object Reference") (OtherComp :type "PrimitiveComponent Object Reference") (OtherBodyIndex :type Integer) (bFromSweep :type Boolean) (SweepResult :type "HitResult Structure (by ref)"))
  (message `/Game/Umit/Blueprints/InteractInterface.InteractAreaEnt` OtherActor self))

(event `self.Trigger.OnComponentEndOverlap`
  (params (OverlappedComponent :type "PrimitiveComponent Object Reference") (OtherActor :type "Actor Object Reference") (OtherComp :type "PrimitiveComponent Object Reference") (OtherBodyIndex :type Integer))
  (message `/Game/Umit/Blueprints/InteractInterface.InteractAreaExt` OtherActor))

(event `/Game/Umit/Blueprints/InteractInterface.Interaction`
  (bind _spotlight (`self.SpotLight`))
  ;[1 1 1] Lights On/Off with Intensity
  (`/Engine/EditorBlueprintResources/StandardMacros.FlipFlop`
    (:`A`
      (`LightComponent.SetIntensity` _spotlight 0.0)
      (`LightComponent.SetIntensity` (`self.SpotLight1`) 0.0)
      (`LightComponent.SetIntensity` (`self.SpotLight2`) 0.0)
      (`LightComponent.SetIntensity` (`self.SpotLight3`) 0.0))
    (:`B`
      (`LightComponent.SetIntensity` _spotlight 5000.0)
      (`LightComponent.SetIntensity` (`self.SpotLight1`) 5000.0)
      (`LightComponent.SetIntensity` (`self.SpotLight2`) 5000.0)
      (`LightComponent.SetIntensity` (`self.SpotLight3`) 5000.0))))

(fn `UserConstructionScript`)