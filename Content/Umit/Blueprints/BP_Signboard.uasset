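; BP_Signboard is a signboard actor that swaps between an info text and a set of Paper sprites based on the player character's State.
; The construction script copies the Info variable into InfoText, and BeginPlay caches the BP_ThirdPersonCharacter and hides both displays.
; Tick polls that State every frame, showing the text for the first enum value and the PaperSpriteList children otherwise.
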(event `self.ReceiveBeginPlay`
  (bind _asbp_third_person_character (cast `/Game/ThirdPerson/Blueprints/BP_ThirdPersonCharacter` (`GameplayStatics.GetPlayerCharacter` 0)))
  (set `self.As BP Third Person Character` _asbp_third_person_character)
  (`SceneComponent.SetHiddenInGame` (`self.InfoText`) true false)
  (for _array_element (`SceneComponent.GetChildrenComponents` (`self.PaperSpriteList`) false)
    (`SceneComponent.SetHiddenInGame` _array_element true false)))

(event `self.ReceiveTick`
  (params (DeltaSeconds :type "Float (single-precision)"))
  (if (`|EnumEquality` (`/Game/ThirdPerson/Blueprints/BP_ThirdPersonCharacter.State` (`self.As BP Third Person Character`)) "NewEnumerator0")
    (for _array_element (`SceneComponent.GetChildrenComponents` (`self.PaperSpriteList`) false)
      (`SceneComponent.SetHiddenInGame` _array_element true false)
      (`SceneComponent.SetHiddenInGame` (`self.InfoText`) false false))
    (else
      (for _array_element_2 (`SceneComponent.GetChildrenComponents` (`self.PaperSpriteList`) false)
        (`SceneComponent.SetHiddenInGame` _array_element_2 false false)
        (`SceneComponent.SetHiddenInGame` (`self.InfoText`) true false)))))

(fn `UserConstructionScript`
  (`TextRenderComponent.K2_SetText` (`self.InfoText`) (`self.Info`)))