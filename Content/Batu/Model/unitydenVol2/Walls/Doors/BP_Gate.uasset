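; Laser security gate that kills the player on contact and can be switched off, with a password prompt nearby.
; Touching LaserBox disables input, shows the Wasted widget, then respawns via the game mode's CheckpointControl after a delay and re-enables input.
; PasswordArea shows an interact prompt for a character in the required state, handing it the gate reference and password.
; DeactiveGate hides the beams and disables both collision volumes, with no caller in this Blueprint.
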(event `self.ReceiveBeginPlay`
  (bind _asbp_third_person_game_mode (cast `/Game/ThirdPerson/Blueprints/BP_ThirdPersonGameMode` (`GameplayStatics.GetGameMode`)))
  (set `self.As BP Third Person Game Mode` _asbp_third_person_game_mode))

(event `self.LaserBox.OnComponentBeginOverlap`
  (params (OverlappedComponent :type "PrimitiveComponent Object Reference") (OtherActor :type "Actor Object Reference") (OtherComp :type "PrimitiveComponent Object Reference") (OtherBodyIndex :type Integer) (bFromSweep :type Boolean) (SweepResult :type "HitResult Structure (by ref)"))
  (bind _asbp_third_person_character (cast `/Game/ThirdPerson/Blueprints/BP_ThirdPersonCharacter` OtherActor))
  (`self.DisableInput` _asbp_third_person_character null)
  (bind _returnvalue (`|CreateWidget` "/Game/ThirdPerson/AI/WBP_Wasted.WBP_Wasted_C"))
  (`UserWidget.AddToViewport` _returnvalue 0)
  (`KismetSystemLibrary.Delay` (`/Game/ThirdPerson/AI/WBP_Wasted.DeathScreenTime` _returnvalue))
  (`/Game/Ozgur/Blueprints/BP_CheckpointControl.Spawn Checkpoint` (`/Game/ThirdPerson/Blueprints/BP_ThirdPersonGameMode.CheckpointControl` (`self.As BP Third Person Game Mode`)))
  (`self.EnableInput` OtherActor null))

(event `self.PasswordArea.OnComponentBeginOverlap`
  (params (OverlappedComponent :type "PrimitiveComponent Object Reference") (OtherActor :type "Actor Object Reference") (OtherComp :type "PrimitiveComponent Object Reference") (OtherBodyIndex :type Integer) (bFromSweep :type Boolean) (SweepResult :type "HitResult Structure (by ref)"))
  (bind _asbp_third_person_character (cast `/Game/ThirdPerson/Blueprints/BP_ThirdPersonCharacter` OtherActor))
  (if (`|EnumEquality` (`/Game/ThirdPerson/Blueprints/BP_ThirdPersonCharacter.State` _asbp_third_person_character) "NewEnumerator0")
    (bind _returnvalue (`|CreateWidget` "/Game/ThirdPerson/Blueprints/DoorSystem/WBP_InteractPassText.WBP_InteractPassText_C"))
    (`UserWidget.AddToViewport` _returnvalue 0)
    (set `/Game/ThirdPerson/Blueprints/BP_ThirdPersonCharacter.CanEnterPassword` true _asbp_third_person_character)
    (set `/Game/ThirdPerson/Blueprints/BP_ThirdPersonCharacter.CurrentActorToInteractWith` self _asbp_third_person_character)
    (set `/Game/ThirdPerson/Blueprints/BP_ThirdPersonCharacter.InteractPass` (`self.Password`) _asbp_third_person_character)))

(event `self.PasswordArea.OnComponentEndOverlap`
  (params (OverlappedComponent :type "PrimitiveComponent Object Reference") (OtherActor :type "Actor Object Reference") (OtherComp :type "PrimitiveComponent Object Reference") (OtherBodyIndex :type Integer))
  (bind _asbp_third_person_character (cast `/Game/ThirdPerson/Blueprints/BP_ThirdPersonCharacter` OtherActor))
  (if (`|EnumEquality` (`/Game/ThirdPerson/Blueprints/BP_ThirdPersonCharacter.State` _asbp_third_person_character) "NewEnumerator0")
    (`/Engine/EditorBlueprintResources/StandardMacros.IsValid` (stale `self.PasswordArea.OnComponentBeginOverlap` _returnvalue)
      (:`Is Valid`
        (`Widget.RemoveFromParent` (stale `self.PasswordArea.OnComponentBeginOverlap` _returnvalue))
        (set `/Game/ThirdPerson/Blueprints/BP_ThirdPersonCharacter.CanEnterPassword` false (stale `self.PasswordArea.OnComponentBeginOverlap` _asbp_third_person_character))))))

(fn `DeactiveGate`
  (`SceneComponent.SetVisibility` (`self.SecruityGate_SecurityGateBeams`) false false)
  (`PrimitiveComponent.SetCollisionEnabled` (`self.LaserBox`) "NoCollision")
  (`PrimitiveComponent.SetCollisionEnabled` (`self.PasswordArea`) "NoCollision"))

(fn `UserConstructionScript`)