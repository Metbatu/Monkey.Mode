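; BP_CheckpointControl tracks the player's last checkpoint and returns the player to it.
; UpdateCheckpoint stores the CheckpointList entry at the current index as LastCheckpoint and increments the index, so checkpoints advance in list order.
; SpawnCheckpoint moves player pawn 0 to that checkpoint's location without sweeping, leaving rotation untouched.
; Both functions rely on outside callers, as the event graph holds only an empty Tick.
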(event `self.ReceiveTick`
  (params (DeltaSeconds :type "Float (single-precision)")))

(fn `Spawn Checkpoint`
  (`self.K2_SetActorLocation` (`GameplayStatics.GetPlayerPawn` 0) (`self.K2_GetActorLocation` (`self.LastCheckpoint`)) false false))

(fn `UpdateCheckpoint`
  (set `self.LastCheckpoint` (`|GetArrayItem` (`self.CheckpointList`) (`self.CheckpointIndex`)))
  (bind _result (`/Engine/EditorBlueprintResources/StandardMacros.IncrementInt` (`self.CheckpointIndex`))
    (:`  `
      (set `self.CheckpointIndex` _result))))

(fn `UserConstructionScript`)