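; Banana pickup actor that the third-person character collects by walking into it.
; When its Box overlaps BP_ThirdPersonCharacter and the character's BananaCounter is below MaxBananaCount, it adds one to the counter, prints the new total, plays an eating sound and destroys itself.
; At the maximum count the banana stays in the level.
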(event `self.Box.OnComponentBeginOverlap`
  (params (OverlappedComponent :type "PrimitiveComponent Object Reference") (OtherActor :type "Actor Object Reference") (OtherComp :type "PrimitiveComponent Object Reference") (OtherBodyIndex :type Integer) (bFromSweep :type Boolean) (SweepResult :type "HitResult Structure (by ref)"))
  (bind _asbp_third_person_character (cast `/Game/ThirdPerson/Blueprints/BP_ThirdPersonCharacter` OtherActor))
  (bind _bananacounter (`/Game/ThirdPerson/Blueprints/BP_ThirdPersonCharacter.BananaCounter` _asbp_third_person_character))
  (if (< _bananacounter (`/Game/ThirdPerson/Blueprints/BP_ThirdPersonCharacter.MaxBananaCount` _asbp_third_person_character))
    (bind _output_get (set `/Game/ThirdPerson/Blueprints/BP_ThirdPersonCharacter.BananaCounter` (+ _bananacounter 1.0) _asbp_third_person_character))
    (`KismetSystemLibrary.PrintString` (`KismetStringLibrary.Conv_DoubleToString` _output_get))
    (`GameplayStatics.PlaySound2D` "/Game/Ozgur/Assets/SoundEffects/eating-sound-effect-36186__online-audio-converter_com_.eating-sound-effect-36186__online-audio-converter_com_" 1.0 1.0 0.0 null null)
    (`self.K2_DestroyActor`)))

(fn `UserConstructionScript`)